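; BP_DoorMiniMarket is an interactable minimarket door that swings open and closed.
; Interact is ignored while the door is locked or moving; otherwise it toggles the open state and plays or reverses a timeline.
; The timeline lerps the Door011 component's relative yaw from zero to Degree, clearing the moving flag when finished.
; Degree is forced positive unless IsInverted is set, which keeps its configured sign.
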(event EventInteract
  (if (Variables|Default|GetisInverted)
    (Variables|Default|SetDegree (Variables|Default|GetDegree))
    (else
      (Variables|Default|SetDegree (Math|Float|Absolute(Float) (Variables|Default|GetDegree)))))
  (if (not (Variables|Default|GetisLocked))
    (if (not (Variables|Default|GetisMoving))
      (Variables|Default|SetisMoving true)
      (bind _output_get (Variables|Default|SetisOpened (not (Variables|Default|GetisOpened))))
      (if _output_get
        (bind _dooralpha (Timeline|TL_Door Play)
          (:Update
            (Transformation|SetRelativeRotation (Variables|Default|GetDoor_011) (Math|Rotator|MakeRotator 0.0 0.0 (Math|Float|Lerp 0.0 (Variables|Default|GetDegree) _dooralpha)) false false))
          (:Finished
            (Variables|Default|SetisMoving false)))
        (else
          (Timeline|TL_Door Reverse))))))

(fn ConstructionScript)