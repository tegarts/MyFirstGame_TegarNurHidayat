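; Interactable, lockable door actor that swings its mesh on yaw through timelines, with an IsMoving guard against re-triggering.
; Interact shows a timed locked widget with sound or toggles the door, PickupKeyItem unlocks it, and other events force its state or snap it open.
; Inner and outer spheres switch two pairs of icons by player proximity.
; The construction script applies per-instance mesh, transform, sphere radii and icon placement, with debug icon visibility.
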(event OnComponentBeginOverlap(InSphere)
  (params (OverlappedComponent :type Primitive%20Component%20Object%20Reference) (OtherActor :type Actor%20Object%20Reference) (OtherComp :type Primitive%20Component%20Object%20Reference) (OtherBodyIndex :type Integer) (bFromSweep :type Boolean) (SweepResult :type Hit%20Result%20Structure%20%28by%20ref%29))
  (if (== (Game|GetPlayerCharacter 0) OtherActor)
    (Rendering|SetVisibility (Variables|Default|GetInner%20A) true false)
    (Rendering|SetVisibility (Variables|Default|GetOuter%20A) false false)))

(event OnComponentEndOverlap(InSphere)
  (params (OverlappedComponent :type Primitive%20Component%20Object%20Reference) (OtherActor :type Actor%20Object%20Reference) (OtherComp :type Primitive%20Component%20Object%20Reference) (OtherBodyIndex :type Integer))
  (if (== OtherActor (Game|GetPlayerCharacter 0))
    (Rendering|SetVisibility (Variables|Default|GetInner%20A) false false)
    (Rendering|SetVisibility (Variables|Default|GetOuter%20B) true false)))

(event OnComponentBeginOverlap(OutSphere)
  (params (OverlappedComponent :type Primitive%20Component%20Object%20Reference) (OtherActor :type Actor%20Object%20Reference) (OtherComp :type Primitive%20Component%20Object%20Reference) (OtherBodyIndex :type Integer) (bFromSweep :type Boolean) (SweepResult :type Hit%20Result%20Structure%20%28by%20ref%29))
  (if (== OtherActor (Game|GetPlayerCharacter 0))
    (Rendering|SetVisibility (Variables|Default|GetOuter%20A) true false)))

(event OnComponentEndOverlap(OutSphere)
  (params (OverlappedComponent :type Primitive%20Component%20Object%20Reference) (OtherActor :type Actor%20Object%20Reference) (OtherComp :type Primitive%20Component%20Object%20Reference) (OtherBodyIndex :type Integer))
  (if (== OtherActor (Game|GetPlayerCharacter 0))
    (Rendering|SetVisibility (Variables|Default|GetOuter%20B) false false)))

(event Custom|ForceInteractDoor
  (params (IsOpening :type Boolean))
  (if (not (Variables|Default|GetisMoving))
    (Variables|Default|SetisMoving true)
    (Audio|PlaySoundatLocation "/Game/Agate/SOund/horror-door-1-453395__mp3cut_net__1_.horror-door-1-453395__mp3cut_net__1_" (Transformation|GetActorLocation) "0, 0, 0" 1.0 1.0 0.0 "/USDCore/USDDefaultAttenuation.USDDefaultAttenuation" 0 0 0)
    (bind _output_get (Variables|Default|SetisOpened IsOpening))
    (if _output_get
      (bind _dooralpha (Timeline|Timeline_0 PlayFromStart)
        (:Update
          (Transformation|SetRelativeRotation (Variables|Default|GetDoor_011) (Math|Rotator|MakeRotator 0.0 0.0 (Math|Float|Lerp 0.0 (Variables|Default|GetDegree) _dooralpha)) false false))
        (:Finished
          (Variables|Default|SetisMoving false)))
      (else
        (Timeline|Timeline_0 ReverseFromEnd)))))

(event Custom|Bathroom%20door
  (Transformation|SetRelativeRotation (Variables|Default|GetDoor_011) "0.000000,103.000000,0.000000" false false)
  (Variables|Default|SetisOpened true))

(event EventPickupKeyItem
  (params (Doors :type BP%20New%20Door%20Object%20Reference))
  (Variables|Default|SetisLocked false))

(event EventInteract
  (params (Character :type BP%20First%20Person%20Character%20Object%20Reference))
  (if (Variables|Default|GetisInverted)
    (Variables|Default|SetDegree (Variables|Default|GetDegree))
    (else
      (Variables|Default|SetDegree (Math|Float|Absolute(Float) (Variables|Default|GetDegree)))))
  (if (Variables|Default|GetisLocked)
    (if (not (Variables|Default|GetIs%20Locked%20Text%20Displayed))
      (Audio|PlaySoundatLocation "/Game/Agate/SOund/the-sound-of-a-locked-door__mp3cut_net__1_.the-sound-of-a-locked-door__mp3cut_net__1_" (Transformation|GetActorLocation) "0, 0, 0" 1.0 1.0 0.0 "/USDCore/USDDefaultAttenuation.USDDefaultAttenuation" 0 0 0)
      (Variables|Default|SetIs%20Locked%20Text%20Displayed true)
      (bind _returnvalue (UserInterface|CreateWidget "/Game/Agate/Widgets/WBP_DoorLocked.WBP_DoorLocked_C"))
      (bind _output_get (Variables|Default|SetLocked%20Widget _returnvalue))
      (UserInterface|Viewport|AddtoViewport _output_get 0)
      (Utilities|Time|SetTimerbyFunctionName 0 "DestroyMyWidget" 1.5))
    (elif (not (Variables|Default|GetisMoving))
      (Audio|PlaySoundatLocation "/Game/Agate/SOund/horror-door-1-453395__mp3cut_net__1_.horror-door-1-453395__mp3cut_net__1_" (Transformation|GetActorLocation) "0, 0, 0" 1.0 1.0 0.0 "/USDCore/USDDefaultAttenuation.USDDefaultAttenuation" 0 0 0)
      (Variables|Default|SetisMoving true)
      (bind _output_get_2 (Variables|Default|SetisOpened (not (Variables|Default|GetisOpened))))
      (if _output_get_2
        (bind _dooralpha (Timeline|TL_Door Play)
          (:Update
            (Transformation|SetRelativeRotation (Variables|Default|GetDoor_011) (Math|Rotator|MakeRotator 0.0 0.0 (Math|Float|Lerp 0.0 (Variables|Default|GetDegree) _dooralpha)) false false))
          (:Finished
            (Variables|Default|SetisMoving false)))
        (else
          (Timeline|TL_Door Reverse))))))

(fn ConstructionScript
  (bind _door_011 (Variables|Default|GetDoor_011))
  (Utilities|FlowControl|Sequence
    (:then_0
      (Components|Sphere|SetSphereRadius (Variables|Default|GetInSphere) (Variables|Default|GetInner%20Sphere%20Radius) true)
      (Components|Sphere|SetSphereRadius (Variables|Default|GetOutSphere) (Variables|Default|GetOuter%20Sphere%20Radius) true))
    (:then_1
      (Components|StaticMesh|SetStaticMesh _door_011 (Variables|Default|GetMesh))
      (Transformation|SetWorldTransform _door_011 (Math|Transform|MakeTransform (+ (Transformation|GetWorldLocation _door_011) (Variables|Default|GetMesh%20Location)) (Transformation|GetWorldRotation _door_011) (Variables|Default|GetMesh%20Scale)) false false))
    (:then_2
      (Transformation|SetRelativeLocation (Variables|Default|GetOuter%20A) (Variables|Default|GetIcon%20Location%20A) false false)
      (Rendering|SetVisibility (Variables|Default|GetInner%20A) (Variables|Default|GetIsDebugging) false))
    (:then_3
      (Transformation|SetRelativeLocation (Variables|Default|GetOuter%20B) (Variables|Default|GetIcon%20Location%20B) false false)
      (Rendering|SetVisibility (Variables|Default|GetInner%20B) (Variables|Default|GetIsDebugging) false))))

(fn DestroyMyWidget
  (Widget|RemovefromParent (Variables|Default|GetLocked%20Widget))
  (Variables|Default|SetLocked%20Widget 0)
  (Variables|Default|SetIs%20Locked%20Text%20Displayed false))