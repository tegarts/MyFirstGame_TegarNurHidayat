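; Restaurant front door Blueprint that swings Door01 open and closed around its yaw using timeline-driven lerps up to Degree.
; Interact toggles the door unless it is locked or moving, forcing a positive angle unless IsInverted is set.
; PickupKeyItem clears the lock, while ForceInteractDoor ignores it and drives a requested state through a separate timeline.
; A third timeline closing branch is left unconnected.
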(event Custom|ForceInteractDoor
  (params (IsOpening :type Boolean))
  (if (not (Variables|Default|GetisMoving))
    (Variables|Default|SetisMoving true)
    (bind _output_get (Variables|Default|SetisOpened IsOpening))
    (if _output_get
      (bind _dooralpha (Timeline|Timeline_0 PlayFromStart)
        (:Update
          (Transformation|SetRelativeRotation (Variables|Default|GetDoor_01) (Math|Rotator|MakeRotator 0.0 0.0 (Math|Float|Lerp 0.0 (Variables|Default|GetDegree) _dooralpha)) false false))
        (:Finished
          (Variables|Default|SetisMoving false)))
      (else
        (Timeline|Timeline_0 ReverseFromEnd)))))

(event EventPickupKeyItem
  (params (Doors :type BP%20Front%20Door%20Restaurant%20Object%20Reference))
  (Variables|Default|SetisLocked false))

(event EventInteract
  (params (Character :type BP%20First%20Person%20Character%20Object%20Reference))
  (if (Variables|Default|GetisInverted)
    (Variables|Default|SetDegree (Variables|Default|GetDegree))
    (else
      (Variables|Default|SetDegree (Math|Float|Absolute(Float) (Variables|Default|GetDegree)))))
  (if (not (Variables|Default|GetisLocked))
    (if (not (Variables|Default|GetisMoving))
      (Variables|Default|SetisMoving true)
      (bind _output_get (Variables|Default|SetisOpened (not (Variables|Default|GetisOpened))))
      (if _output_get
        (bind _dooralpha (Timeline|TL_Door Play)
          (:Update
            (Transformation|SetRelativeRotation (Variables|Default|GetDoor_01) (Math|Rotator|MakeRotator 0.0 0.0 (Math|Float|Lerp 0.0 (Variables|Default|GetDegree) _dooralpha)) false false))
          (:Finished
            (Variables|Default|SetisMoving false)))
        (else
          (Timeline|TL_Door Reverse))))))

(fn ConstructionScript)