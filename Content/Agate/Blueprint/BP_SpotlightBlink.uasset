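; BP_SpotlightBlink is a spotlight Blueprint that blinks on and off at random intervals.
; BeginPlay starts the Blink event, which uses a FlipFlop to alternate the SpotLight between zero and NewIntensity, starting dark.
; After each switch it waits a random delay between MinRange and MaxRange, then calls itself again to loop indefinitely.
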(event Custom|Blink
  (bind _spotlight (Variables|Default|GetSpotLight))
  (bind _minrange (Variables|Default|GetMinRange))
  (bind _maxrange (Variables|Default|GetMaxRange))
  (bind _returnvalue (Math|Random|RandomFloatinRange _minrange _maxrange))
  (Utilities|FlowControl|FlipFlop
    (:A
      (Rendering|Components|Light|SetIntensity _spotlight 0.0)
      (Utilities|FlowControl|Delay _returnvalue)
      (CallFunction|Blink))
    (:B
      (Rendering|Components|Light|SetIntensity _spotlight (Variables|Default|GetNewIntensity))
      (Utilities|FlowControl|Delay _returnvalue)
      (CallFunction|Blink))))

(event EventBeginPlay
  (CallFunction|Blink))

(fn ConstructionScript)