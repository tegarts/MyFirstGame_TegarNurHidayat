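; Spotlight actor Blueprint that makes two spotlights blink irregularly with a car alarm sound.
; A custom Blink event uses a FlipFlop to alternate both lights between zero and a set intensity, waits a random delay within a min/max range, then calls itself again.
; Each switch-on plays the loud, attenuated alarm at the actor's location.
; Nothing in this graph makes the initial Blink call.
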(event Custom|Blink
  (bind _minrange (Variables|Default|GetMinRange))
  (bind _maxrange (Variables|Default|GetMaxRange))
  (bind _spotlight (Variables|Default|GetSpotLight))
  (bind _returnvalue (Math|Random|RandomFloatinRange _minrange _maxrange))
  (Utilities|FlowControl|FlipFlop
    (:A
      (Rendering|Components|Light|SetIntensity _spotlight 0.0)
      (Utilities|FlowControl|Delay _returnvalue)
      (CallFunction|Blink))
    (:B
      (Audio|PlaySoundatLocation "/Game/Agate/SOund/car-alarm-raw-43056__mp3cut_net_.car-alarm-raw-43056__mp3cut_net_" (Transformation|GetActorLocation) "0, 0, 0" 5.0 1.0 0.0 "/USDCore/USDDefaultAttenuation.USDDefaultAttenuation" 0 0 0)
      (Rendering|Components|Light|SetIntensity _spotlight (Variables|Default|GetNewIntensity))
      (Utilities|FlowControl|Delay _returnvalue)
      (CallFunction|Blink))))

(fn ConstructionScript)