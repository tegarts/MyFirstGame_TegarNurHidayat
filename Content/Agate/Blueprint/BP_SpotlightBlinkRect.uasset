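; BP_SpotlightBlinkRect is a rect light Blueprint that flickers on and off at random intervals.
; Its Blink event uses a FlipFlop to alternate between zero and a set intensity, playing a quiet lamp switch sound at each switch-on.
; After a random delay, Blink calls itself again until the light is hidden in game; nothing in this graph makes the first call.
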(event Custom|Blink
  (bind _minrange (Variables|Default|GetMinRange))
  (bind _maxrange (Variables|Default|GetMaxRange))
  (bind _rectlight (Variables|Default|GetRectLight))
  (bind _returnvalue (Math|Random|RandomFloatinRange _minrange _maxrange))
  (Utilities|FlowControl|FlipFlop
    (:A
      (Rendering|Components|Light|SetIntensity _rectlight 0.0)
      (Utilities|FlowControl|Delay _returnvalue)
      (if (not (Variables|/Script/Engine.SceneComponent|GetbHiddenInGame (Variables|Default|GetRectLight)))
        (CallFunction|Blink)))
    (:B
      (Audio|PlaySoundatLocation "/Game/Agate/SOund/desk-lamp-switch-turned-on-amp-off-384165__mp3cut_net_.desk-lamp-switch-turned-on-amp-off-384165__mp3cut_net_" (Transformation|GetActorLocation) "0, 0, 0" 0.2 1.0 0.0 "/USDCore/USDDefaultAttenuation.USDDefaultAttenuation" 0 0 0)
      (Rendering|Components|Light|SetIntensity _rectlight (Variables|Default|GetNewIntensity))
      (Utilities|FlowControl|Delay _returnvalue)
      (if (not (Variables|/Script/Engine.SceneComponent|GetbHiddenInGame (Variables|Default|GetRectLight)))
        (CallFunction|Blink)))))

(fn ConstructionScript)