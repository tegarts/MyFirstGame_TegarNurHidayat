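; Interactable mini market door that swings Door011 open and closed unless locked.
; Interact toggles IsOpened and plays or reverses a timeline that lerps yaw to Degree, with IsMoving blocking re-triggers mid-swing.
; Degree is forced positive unless IsInverted is set.
; Two overlap spheres swap component visibility for the player: OutSphere reveals the Outer pair, while InSphere shows the Inner pair in its place.
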(event OnComponentBeginOverlap(InSphere)
  (params (OverlappedComponent :type Primitive%20Component%20Object%20Reference) (OtherActor :type Actor%20Object%20Reference) (OtherComp :type Primitive%20Component%20Object%20Reference) (OtherBodyIndex :type Integer) (bFromSweep :type Boolean) (SweepResult :type Hit%20Result%20Structure%20%28by%20ref%29))
  (if (== (Game|GetPlayerCharacter 0) OtherActor)
    (Rendering|SetVisibility (Variables|Default|GetInner%20A) true false)
    (Rendering|SetVisibility (Variables|Default|GetOuter%20A) false false)))

(event OnComponentEndOverlap(InSphere)
  (params (OverlappedComponent :type Primitive%20Component%20Object%20Reference) (OtherActor :type Actor%20Object%20Reference) (OtherComp :type Primitive%20Component%20Object%20Reference) (OtherBodyIndex :type Integer))
  (if (== OtherActor (Game|GetPlayerCharacter 0))
    (Rendering|SetVisibility (Variables|Default|GetInner%20A) false false)
    (Rendering|SetVisibility (Variables|Default|GetOuter%20B) true false)))

(event OnComponentBeginOverlap(OutSphere)
  (params (OverlappedComponent :type Primitive%20Component%20Object%20Reference) (OtherActor :type Actor%20Object%20Reference) (OtherComp :type Primitive%20Component%20Object%20Reference) (OtherBodyIndex :type Integer) (bFromSweep :type Boolean) (SweepResult :type Hit%20Result%20Structure%20%28by%20ref%29))
  (if (== OtherActor (Game|GetPlayerCharacter 0))
    (Rendering|SetVisibility (Variables|Default|GetOuter%20A) true false)))

(event OnComponentEndOverlap(OutSphere)
  (params (OverlappedComponent :type Primitive%20Component%20Object%20Reference) (OtherActor :type Actor%20Object%20Reference) (OtherComp :type Primitive%20Component%20Object%20Reference) (OtherBodyIndex :type Integer))
  (if (== OtherActor (Game|GetPlayerCharacter 0))
    (Rendering|SetVisibility (Variables|Default|GetOuter%20B) false false)))

(event EventInteract
  (if (Variables|Default|GetisInverted)
    (Variables|Default|SetDegree (Variables|Default|GetDegree))
    (else
      (Variables|Default|SetDegree (Math|Float|Absolute(Float) (Variables|Default|GetDegree)))))
  (if (not (Variables|Default|GetisLocked))
    (if (not (Variables|Default|GetisMoving))
      (Variables|Default|SetisMoving true)
      (bind _output_get (Variables|Default|SetisOpened (not (Variables|Default|GetisOpened))))
      (if _output_get
        (bind _dooralpha (Timeline|TL_Door Play)
          (:Update
            (Transformation|SetRelativeRotation (Variables|Default|GetDoor_011) (Math|Rotator|MakeRotator 0.0 0.0 (Math|Float|Lerp 0.0 (Variables|Default|GetDegree) _dooralpha)) false false))
          (:Finished
            (Variables|Default|SetisMoving false)))
        (else
          (Timeline|TL_Door Reverse))))))

(fn ConstructionScript)